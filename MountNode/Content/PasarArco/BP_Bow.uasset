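; VR bow whose string, once grabbing is allowed, is drawn with a motion controller to shoot arrows.
; While held, a looping timer follows the controller along the string's local Y, clamped between two spline points, and normalizes it into PullBack.
; Release resets the string, spawns Projectile_Arrow with PullBack as speed input, and fires a first-shot event once.
; BeginPlay finds the tutorial actor but only unbinds the CanGrab-enabling event from its audio-finished dispatcher.
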(event `self.ReceiveBeginPlay`
  (bind _returnvalue (`GameplayStatics.GetActorOfClass` "/Game/BluePrints/BP_IA_Tutorial.BP_IA_Tutorial_C"))
  (set `self.IATutorialRef` _returnvalue)
  (`self.OnEnable`))

(event `OnEnable`
  (remove `/Game/BluePrints/BP_IA_Tutorial.AudioTutorial03Finished` (`self.IATutorialRef`) (delegate `CustomEvent`)))

(event `CustomEvent`
  (set `self.CanGrab` true))

(event `self.GrabString.OnGrabbed`
  (params (`Motion Controller` :type "MotionControllerComponent Object Reference"))
  (if (`self.CanGrab`)
    (`|ExecutionSequence`
      (:`then_0`
        (set `self.Motion Controller` `Motion Controller`)
        (`SceneComponent.SetVisibility` (`self.Arrow`) true false)
        (bind _returnvalue (`KismetSystemLibrary.K2_SetTimer` null "RelativePosition" 0.01 true))
        (set `self.Timer` _returnvalue))
      (:`then_1`
        (set `self.isGrabbingBow` true)))))

(event `self.GrabString.OnDropped`
  (bind _arrowspawnpoint (`self.ArrowSpawnPoint`))
  (`|ExecutionSequence`
    (:`then_0`
      (`KismetSystemLibrary.K2_ClearAndInvalidateTimerHandle` (`self.Timer`))
      (set `self.Motion Controller` null)
      (`SceneComponent.K2_SetRelativeLocation` (`self.ColliderString`) (0.0 170.0 0.0) false true)
      (`SceneComponent.SetVisibility` (`self.Arrow`) false false))
    (:`then_1`
      (bind _returnvalue (`|SpawnActorFromClass` "/Game/PasarArco/Projectile_Arrow.Projectile_Arrow_C" (`KismetMathLibrary.MakeTransform` (`SceneComponent.K2_GetComponentLocation` _arrowspawnpoint) (`SceneComponent.K2_GetComponentRotation` _arrowspawnpoint)) "Undefined" "MultiplyWithRoot" self (`GameplayStatics.GetPlayerPawn` 0)))
      (`|ExecutionSequence`
        (:`then_0`
          (`/Game/PasarArco/Projectile_Arrow.ArrowSpeed   ` _returnvalue (`self.PullBack`)))
        (:`then_1`
          (`/Engine/EditorBlueprintResources/StandardMacros.DoOnce` false
            (:`Completed`
              (`|ExecutionSequence`
                (:`then_0`
                  (set `self.CanGrab` true))
                (:`then_1`
                  (`self.PlayerFisrtShoot`))))))))
    (:`then_2`
      (set `self.PullBack` 0.0))
    (:`then_3`
      (set `self.isGrabbingBow` false))))

(fn `RelativePosition`
  (bind _spline (`self.Spline`))
  (bind (_returnvalue_x _returnvalue_y) (`KismetMathLibrary.BreakVector` (`SplineComponent.GetLocationAtSplinePoint` _spline 1 "Local")))
  (bind (_returnvalue_x_2 _returnvalue_y_2) (`KismetMathLibrary.BreakVector` (`SplineComponent.GetLocationAtSplinePoint` _spline 0 "Local")))
  (bind (_relativelocation_x _relativelocation_y) (`KismetMathLibrary.BreakVector` (`SceneComponent.RelativeLocation` (`self.ColliderString`))))
  (bind _returnvalue (`KismetMathLibrary.FClamp` (+ (.y (.location (`KismetMathLibrary.MakeRelativeTransform` (`SceneComponent.K2_GetComponentToWorld` (`self.Motion Controller`)) (`SceneComponent.K2_GetComponentToWorld` (`self.ColliderString`))))) _relativelocation_y) _returnvalue_y_2 _returnvalue_y))
  (`SceneComponent.K2_SetRelativeLocation` (`self.ColliderString`) (`KismetMathLibrary.MakeVector` 0.0 _returnvalue) false true)
  (set `self.PullBack` (`KismetMathLibrary.NormalizeToRange` _returnvalue _returnvalue_y_2 _returnvalue_y)))

(fn `UserConstructionScript`)