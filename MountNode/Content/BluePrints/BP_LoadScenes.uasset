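; BP_LoadScenes is a trigger box that marks the dragon player's arrival at the clouds.
; It caches the VRPawn1 reference one second after BeginPlay.
; When a component tagged DragonCollider overlaps the box, it sets FinalClouds, disables movement, zeroes the dragon mesh's physics velocity and prints a debug message.
; Despite the name, it loads no scenes: the old level-streaming switch to the clouds tunnel is left disconnected.
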(event `self.ReceiveBeginPlay`
  (`KismetSystemLibrary.Delay` 1.0)
  (`|ExecutionSequence`
    (:`then_0`
      (bind _returnvalue (`GameplayStatics.GetActorOfClass` "/Game/VRTemplate/Blueprints/VRPawn1.VRPawn1_C"))
      (set `self.As VRPawn 1` _returnvalue))))

(event `self.Box.OnComponentBeginOverlap`
  (params (OverlappedComponent :type "PrimitiveComponent Object Reference") (OtherActor :type "Actor Object Reference") (OtherComp :type "PrimitiveComponent Object Reference") (OtherBodyIndex :type Integer) (bFromSweep :type Boolean) (SweepResult :type "HitResult Structure (by ref)"))
  (bind _as_vrpawn_1 (`self.As VRPawn 1`))
  (if (`ActorComponent.ComponentHasTag` OtherComp "DragonCollider")
    (`|ExecutionSequence`
      (:`then_0`
        (set `/Game/VRTemplate/Blueprints/VRPawn1.FinalClouds` true _as_vrpawn_1))
      (:`then_1`
        (set `/Game/VRTemplate/Blueprints/VRPawn1.CanMove` false _as_vrpawn_1))
      (:`then_2`
        (`KismetSystemLibrary.PrintString` "EL JUGADOR HA TOCADO NUBES"))
      (:`then_3`
        (`PrimitiveComponent.SetAllPhysicsLinearVelocity` (`/Game/VRTemplate/Blueprints/VRPawn1.SK_MOUNTAIN_DRAGON` _as_vrpawn_1) (0.0 0.0 0.0) false)))))

(fn `UserConstructionScript`)