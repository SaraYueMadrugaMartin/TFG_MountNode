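; Tutorial guide NPC that plays a spoken intro at BeginPlay, then leads the player along a spline path.
; Once the first audio ends, Tick drives a timeline whose alpha maps to spline distance and checks player proximity.
; At stop points it pauses until the player is close, then advances to the next.
; FinishTutorial01 plays the next dialogue; idle-wait behavior is an empty stub.
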(event `self.ReceiveBeginPlay`
  ;[0.09375 1 0.1203] START
  (`self.PlayTutoAudios`))

(event `self.ReceiveTick`
  (params (DeltaSeconds :type "Float (single-precision)"))
  ;[0.2969 0.67 1] UPDATE
  (if (`self.Dialogue01Finished`)
    (`|ExecutionSequence`
      (:`then_0`
        (`self.TutorialPath`))
      (:`then_1`
        (`self.CheckPlayerDistance`)))))

(event `PlayTutoAudios`
  ;[1 1 1] Play Tuto Audios
  (bind _returnvalue (`GameplayStatics.SpawnSoundAttached` (`|GetArrayItem` (`self.TutorialsDialogue`) (`self.CurrentAudioIndex`)) (`self.DefaultSceneRoot`) "None" (`SceneComponent.K2_GetComponentLocation` (`self.Cube`)) (struct) "KeepRelativeOffset" false 1.0 1.0 0.0 null null))
  (bind _output_get (set `self.AudioTutorial` _returnvalue))
  (add `AudioComponent.OnAudioFinished` _output_get (delegate `OnAudioFinished_Event_0`))
  (set `self.CurrentAudioIndex` (+ (`self.CurrentAudioIndex`) 1)))

(event `OnAudioFinished_Event_0`
  ;[1 1 1] Play Tuto Audios
  (set `self.Dialogue01Finished` true)
  (`KismetSystemLibrary.PrintString` "¡Primer audio terminado!"))

(event `TutorialPath`
  (bind _npc_path (`/Game/BP_Path.NPC_Path` (`self.Path`)))
  ;[1 1 1] Tutorial Path
  (`TimelineComponent.SetPlayRate` (`self.Timeline Tutorial Path`) (/ 1.0 (`self.TimeCompletePath`)))
  (`self.MoveToStopPoint`)
  (if (`self.IsWaiting`)
    (bind (_direction _newtrack_0) (`Timeline|Timeline Tutorial Path` :!via `Stop` :!label _label)
      (:`Update`
        (`self.K2_SetActorLocationAndRotation` (`SplineComponent.GetLocationAtDistanceAlongSpline` _npc_path (`KismetMathLibrary.Lerp` 0.0 (`SplineComponent.GetSplineLength` _npc_path) _newtrack_0) "World"))))
    (else
      (goto _label))))

(event `MoveToStopPoint`
  ;[1 1 1] Move To Stop Point
  (set `self.StopPointDistance` (`self.GetDistanceTo` self (`|GetArrayItem` (`self.StopPoints`) (`self.CurrentStopPointIndex`))))
  (if (<= (`self.StopPointDistance`) (`self.MaxDistanceStopPoints`))
    (if (`self.PlayerIsClose`)
      (set `self.IsWaiting` false)
      (set `self.CurrentStopPointIndex` (+ (`self.CurrentStopPointIndex`) 1))
      (`self.MoveToStopPoint`)
      (else
        (set `self.IsWaiting` true)
        (set `self.CurrentTimeWaiting` 0.0)
        (`KismetSystemLibrary.K2_SetTimerDelegate` :`Time` 1.0)))))

(event `TimeWaitingPlayer`
  (set `self.CurrentTimeWaiting` (+ (`self.CurrentTimeWaiting`) 1.0)))

(event `CheckPlayerDistance`
  ;[1 1 1] Check Player Distance
  (bind _output_get (set `self.PlayerDistance` (`self.GetDistanceTo` (`GameplayStatics.GetPlayerPawn` 0) self)))
  (if (<= (`self.PlayerDistance`) (`self.MaxDistancePlayer`))
    (set `self.PlayerIsClose` true)
    (else
      (set `self.PlayerIsClose` false))))

(event `FinishTutorial01`
  (`KismetSystemLibrary.PrintString` "¡Empieza el tutorial 2!")
  (`self.PlayTutoAudios`))

(event `IdleWaitingPlayer`
  (if (`self.IsWaiting`)
    _))

(fn `UserConstructionScript`)