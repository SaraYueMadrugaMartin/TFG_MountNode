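; BP_Souls is a soul pickup actor that flies to the player and shrinks away when a Projectile_Arrow overlaps it.
; The overlap prints a debug message, then SoulCatched snapshots the soul's location and scale and the player pawn's location.
; The Souls timeline lerps position toward that captured player location, without tracking later movement, while scaling down to zero; the graph never destroys the actor.
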(event `self.ReceiveActorBeginOverlap`
  (params (OtherActor :type "Actor Object Reference"))
  (bind _asprojectile_arrow (cast `/Game/PasarArco/Projectile_Arrow` OtherActor))
  (`KismetSystemLibrary.PrintString` (`KismetStringLibrary.Concat_StrStr` (`KismetSystemLibrary.GetDisplayName` _asprojectile_arrow) "TOCADO"))
  (`self.SoulCatched`))

(event `SoulCatched`
  (`self.GetTransformSouls`)
  (bind (_direction _tiempo) (`Timeline|Souls` :!via `PlayFromStart`)
    (:`Update`
      (`self.K2_SetActorLocation` (`KismetMathLibrary.VLerp` (`self.StartPos`) (`self.PlayerPos`) _tiempo))
      (`self.SetActorScale3D` (`KismetMathLibrary.VLerp` (`self.StartScale`) (0.0 0.0 0.0) _tiempo)))))

(event `GetTransformSouls`
  (`|ExecutionSequence`
    (:`then_0`
      (set `self.StartPos` (`self.K2_GetActorLocation`)))
    (:`then_1`
      (set `self.PlayerPos` (`self.K2_GetActorLocation` (`GameplayStatics.GetPlayerPawn` 0))))
    (:`then_2`
      (set `self.StartScale` (`self.GetActorScale3D`)))))

(fn `UserConstructionScript`)